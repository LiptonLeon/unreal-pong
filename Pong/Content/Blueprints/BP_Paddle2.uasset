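; BP_Paddle2 is a physics-driven paddle controlled by the P2_AXIS input, apparently for the second player.
; Every Tick it applies a strong force to its static mesh along world X, scaled by the axis value.
; An unconnected chain meant to clamp the actor's X position within roughly ±350 never runs, so this Blueprint enforces no movement limit.
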(event EventBeginPlay)

(event Collision|EventActorBeginOverlap
  (params (OtherActor :type Actor%20Object%20Reference)))

(event EventTick
  (params (DeltaSeconds :type Float%20%28single-precision%29))
  (Physics|AddForce (Variables|Default|GetStaticMesh) (Math|Vector|MakeVector (* (Input|AxisValues|GetP2_AXIS) 2e+06) 0.0 0.0) "None" false))

(fn ConstructionScript)