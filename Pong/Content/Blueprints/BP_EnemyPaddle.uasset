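; BP_EnemyPaddle is the AI-controlled paddle that chases the ball in a Pong game.
; On BeginPlay it caches a ball reference and, outside the main menu, takes its speed from PongGameInstance's BotSpeed.
; Each Tick, for every ball beyond a small X dead zone, it applies a mesh impulse proportional to the offset and speed.
; It then calls the cached ball's UnstuckP1 or UnstuckP2, depending on its side.
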(event EventBeginPlay
  (if (Variables|Default|GetIsMainmenu)
    _
    (else
      (bind _aspong_game_instance (Utilities|Casting|CastToPongGameInstance (Game|GetGameInstance)))
      (Variables|Default|SetSpeed (Variables|/Game/Blueprints/PongGameInstance.PongGameInstance_C|GetBotSpeed _aspong_game_instance))))
  (bind _outactors (Actor|GetAllActorsOfClass "/Game/Blueprints/BP_Ball.BP_Ball_C"))
  (for _array_element _outactors
    (Variables|Default|SetBallRef _array_element)))

(event Collision|EventActorBeginOverlap
  (params (OtherActor :type Actor%20Object%20Reference)))

(event EventTick
  (params (DeltaSeconds :type Float%20%28single-precision%29))
  (bind _outactors (Actor|GetAllActorsOfClass "/Game/Blueprints/BP_Ball.BP_Ball_C"))
  (for _array_element _outactors
    (bind _asbp_ball (Utilities|Casting|CastToBP_Ball _array_element))
    (Math|Float|CompareFloat (Math|Float|Absolute(Float) (- (.X (Math|Vector|BreakVector (Transformation|GetActorLocation _asbp_ball))) (.X (Math|Vector|BreakVector (Transformation|GetActorLocation))))) 2e+01
      (:>
        (Physics|AddImpulse (Variables|Default|GetStaticMesh) (Math|Vector|MakeVector (* (- (.X (Math|Vector|BreakVector (Transformation|GetActorLocation _asbp_ball))) (.X (Math|Vector|BreakVector (Transformation|GetActorLocation)))) (Variables|Default|GetSpeed)) 0.0 0.0) "None" false)
        (if (Variables|Default|GetIsRightSide)
          (Default|UnstuckP2 (Variables|Default|GetBallRef))
          (else
            (Default|UnstuckP1 (Variables|Default|GetBallRef))))))))

(fn ConstructionScript)