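; Player 1's paddle, which moves along the X axis and works with a BP_Ball actor.
; BeginPlay caches a BP_Ball reference from the level.
; Each Tick applies a physics force to the StaticMesh scaled by the P1 axis input, and calls UnstuckP1 on the ball while that input is non-zero.
; A position clamp for the X bounds exists but is disconnected and never runs.
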(event EventBeginPlay
  (bind _outactors (Actor|GetAllActorsOfClass "/Game/Blueprints/BP_Ball.BP_Ball_C"))
  (for _array_element _outactors
    (Variables|Default|SetBallRef _array_element)))

(event Collision|EventActorBeginOverlap
  (params (OtherActor :type Actor%20Object%20Reference)))

(event EventTick
  (params (DeltaSeconds :type Float%20%28single-precision%29))
  (Physics|AddForce (Variables|Default|GetStaticMesh) (Math|Vector|MakeVector (* (Input|AxisValues|GetP1_AXIS) 2e+06) 0.0 0.0) "None" false)
  (if (!= (Input|AxisValues|GetP1_AXIS) 0.0)
    (Default|UnstuckP1 (Variables|Default|GetBallRef))))

(fn ConstructionScript)