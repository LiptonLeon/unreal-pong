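; Pong ball that bounces between paddles and walls, keeps both players' scores and ends the match.
; On overlap, it flips Y off player or enemy paddles, setting X from hit offset, paddle velocity and randomness, and flips X off horizontal walls.
; Goals reset and relaunch it, updating tagged TextRenderActor scores.
; At three points it flags game over, which Tick uses to stop it and load MainMenu after a delay.
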(event EventBeginPlay
  (Physics|SetPhysicsLinearVelocity (Variables|Default|GetStaticMesh) "0.000000,800.000000, 0" false "None"))

(event Collision|EventActorBeginOverlap
  (params (OtherActor :type Actor%20Object%20Reference))
  (bind _staticmesh (Variables|Default|GetStaticMesh))
  (bind _asbp_paddle (Utilities|Casting|CastToBP_Paddle OtherActor)
    (:then
      (bind _returnvalue (Physics|GetPhysicsLinearVelocity (Variables|/Game/Blueprints/BP_Paddle.BP_Paddle_C|GetStaticMesh _asbp_paddle) "None"))
      (bind _returnvalue_2 (Physics|GetPhysicsLinearVelocity (Variables|Default|GetStaticMesh) "None"))
      (Physics|SetPhysicsLinearVelocity (Variables|Default|GetStaticMesh) (Math|Vector|MakeVector (+ (* (- (.X (Math|Vector|BreakVector (Transformation|GetActorLocation))) (.X (Math|Vector|BreakVector (Transformation|GetActorLocation _asbp_paddle)))) 4.0) (* (.X (Math|Vector|BreakVector _returnvalue)) 0.75) (Math|Random|RandomFloatinRange -1e+02 1e+02)) (* (.Y (Math|Vector|BreakVector _returnvalue_2)) -1.0) (.Z (Math|Vector|BreakVector _returnvalue_2))) false "None")
      (Audio|PlaySound2D "/Game/SFX/hit.hit" 1.0 1.0 0.0 0 0 :!label _label))
    (:CastFailed
      (bind _asbp_enemy_paddle (Utilities|Casting|CastToBP_EnemyPaddle OtherActor)
        (:then
          (bind _returnvalue_3 (Physics|GetPhysicsLinearVelocity (Variables|/Game/Blueprints/BP_EnemyPaddle.BP_EnemyPaddle_C|GetStaticMesh _asbp_enemy_paddle) "None"))
          (bind _returnvalue_4 (Physics|GetPhysicsLinearVelocity (Variables|Default|GetStaticMesh) "None"))
          (Physics|SetPhysicsLinearVelocity (Variables|Default|GetStaticMesh) (Math|Vector|MakeVector (+ (* (- (.X (Math|Vector|BreakVector (Transformation|GetActorLocation))) (.X (Math|Vector|BreakVector (Transformation|GetActorLocation _asbp_enemy_paddle)))) 4.0) (* (.X (Math|Vector|BreakVector _returnvalue_3)) 0.75) (Math|Random|RandomFloatinRange -1e+02 1e+02)) (* (.Y (Math|Vector|BreakVector _returnvalue_4)) -1.0) (.Z (Math|Vector|BreakVector _returnvalue_4))) false "None")
          (goto _label))
        (:CastFailed
          (bind _asbp_paddle_2 (Utilities|Casting|CastToBP_Paddle2 OtherActor)
            (:then
              (bind _returnvalue_5 (Physics|GetPhysicsLinearVelocity (Variables|/Game/Blueprints/BP_Paddle2.BP_Paddle2_C|GetStaticMesh _asbp_paddle_2) "None"))
              (bind _returnvalue_6 (Physics|GetPhysicsLinearVelocity (Variables|Default|GetStaticMesh) "None"))
              (Physics|SetPhysicsLinearVelocity (Variables|Default|GetStaticMesh) (Math|Vector|MakeVector (+ (* (- (.X (Math|Vector|BreakVector (Transformation|GetActorLocation))) (.X (Math|Vector|BreakVector (Transformation|GetActorLocation _asbp_paddle_2)))) 4.0) (* (.X (Math|Vector|BreakVector _returnvalue_5)) 0.75) (Math|Random|RandomFloatinRange -1e+02 1e+02)) (* (.Y (Math|Vector|BreakVector _returnvalue_6)) -1.0) (.Z (Math|Vector|BreakVector _returnvalue_6))) false "None")
              (goto _label))
            (:CastFailed
              (bind _asbp_horizontal_wall (Utilities|Casting|CastToBP_HorizontalWall OtherActor)
                (:then
                  (Physics|GetPhysicsLinearVelocity (Variables|/Game/Blueprints/BP_HorizontalWall.BP_HorizontalWall_C|GetStaticMesh _asbp_horizontal_wall) "None")
                  (bind _returnvalue_7 (Physics|GetPhysicsLinearVelocity (Variables|Default|GetStaticMesh) "None"))
                  (Physics|SetPhysicsLinearVelocity (Variables|Default|GetStaticMesh) (Math|Vector|MakeVector (* (.X (Math|Vector|BreakVector _returnvalue_7)) -1.0) (.Y (Math|Vector|BreakVector _returnvalue_7)) (.Z (Math|Vector|BreakVector _returnvalue_7))) false "None")
                  (goto _label))
                (:CastFailed
                  (Utilities|Casting|CastToBP_L_Goal OtherActor
                    (:then
                      (Physics|SetPhysicsLinearVelocity _staticmesh "0,800.000000, 0" false "None")
                      (Transformation|SetWorldLocation _staticmesh "0, 0, 0" false false)
                      (Variables|Default|SetP2_Score (+ (Variables|Default|GetP2_Score) 1))
                      (bind _outactors (Actor|GetAllActorsOfClass "/Script/Engine.TextRenderActor"))
                      (for _array_element _outactors
                        (if (Components|ComponentHasTag (Variables|/Script/Engine.Actor|GetRootComponent _array_element) "P2")
                          (Rendering|Components|TextRender|SetText (Variables|/Script/Engine.TextRenderActor|GetTextRender _array_element) (Utilities|Text|ToText(Integer) (Variables|Default|GetP2_Score)))
                          (if (> (Variables|Default|GetP2_Score) 2)
                            (Development|PrintString "Lost gaem")
                            (Variables|Default|SetisGameover true)
                            (Audio|PlaySound2D "/Game/SFX/gameover.gameover" 1.0 1.0 0.0 0 0)
                            (else
                              (Audio|PlaySound2D "/Game/SFX/score.score" 1.0 1.0 0.0 0 0))))))
                    (:CastFailed
                      (Utilities|Casting|CastToBP_R_Goal OtherActor)
                      (Physics|SetPhysicsLinearVelocity _staticmesh "0,-800.000000, 0" false "None")
                      (Transformation|SetWorldLocation _staticmesh "0, 0, 0" false false)
                      (Variables|Default|SetP1_Score (+ (Variables|Default|GetP1_Score) 1))
                      (bind _outactors_2 (Actor|GetAllActorsOfClass "/Script/Engine.TextRenderActor"))
                      (for _array_element_2 _outactors_2
                        (if (Components|ComponentHasTag (Variables|/Script/Engine.Actor|GetRootComponent _array_element_2) "P1")
                          (Rendering|Components|TextRender|SetText (Variables|/Script/Engine.TextRenderActor|GetTextRender _array_element_2) (Utilities|Text|ToText(Integer) (Variables|Default|GetP1_Score)))
                          (if (> (Variables|Default|GetP1_Score) 2)
                            (Development|PrintString "Victory royale!")
                            (Variables|Default|SetisGameover true)
                            (Audio|PlaySound2D "/Game/SFX/gameover.gameover" 1.0 1.0 0.0 0 0)
                            (else
                              (Audio|PlaySound2D "/Game/SFX/score.score" 1.0 1.0 0.0 0 0))))))))))))))))

(event EventTick
  (params (DeltaSeconds :type Float%20%28single-precision%29))
  (if (Variables|Default|GetisGameover)
    (Physics|SetPhysicsLinearVelocity (Variables|Default|GetStaticMesh) "0, 0, 0" false "None")
    (Utilities|FlowControl|Delay 7.0)
    (Game|OpenLevel(byName) "MainMenu")))

(fn ConstructionScript)